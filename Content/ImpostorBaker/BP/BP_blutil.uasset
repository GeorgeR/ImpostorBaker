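; BP_blutil is a small utility Blueprint for locating and offsetting a streaming level.
; The getlevel event derives a package name from an Actor's path, prints it and stores the matching streaming level.
; The offset event overwrites that level's transform with a fixed shift along X.
; An unconnected node for creating a new streaming level remains in the graph and never runs.
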(event Custom|get%20level
  (bind _actor (Variables|Default|Getactor))
  (bind _returnvalue (Class|KismetSystemLibrary|GetPathName _actor))
  (bind _returnvalue_2 (Utilities|String|ParseIntoArray _returnvalue "."))
  (bind _output (Utilities|Array|Get(acopy) _returnvalue_2))
  (bind _returnvalue_3 (Utilities|String|StringToName _output))
  (Variables|Default|Setlevel (Class|GameplayStatics|GetStreamingLevel _returnvalue_3))
  (Development|PrintString (Utilities|String|ToString(Name) _returnvalue_3)))

(event Custom|offset
  (Variables|/Script/Engine.LevelStreaming|SetLevelTransform (Variables|Default|Getlevel) (Math|Transform|MakeTransform "1000.000000, 0, 0")))

(fn ConstructionScript)