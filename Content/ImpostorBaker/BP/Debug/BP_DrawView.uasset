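; BP_DrawView is an Impostor Baker debug actor that visualizes a view direction V in the world.
; Its construction script flushes persistent debug lines, then draws a long-lived line along normalized V between distances S and L.
; It adds a static mesh just past the line's end, rotated to that direction and offset down its local Z.
; It also writes fixed capture values to MPC_ImposterCapture, enabling capture with depth, radius and unit axis vectors.
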(event EventBeginPlay)

(event Collision|EventActorBeginOverlap
  (params (OtherActor :type Actor%20Object%20Reference)))

(event EventTick
  (params (DeltaSeconds :type Float%20%28single-precision%29)))

(fn ConstructionScript
  (bind _returnvalue (Math|Vector|MakeVector 0.0 0.0 1.0))
  (bind _v (Variables|Default|GetV))
  (bind _l (Variables|Default|GetL))
  (bind _returnvalue_2 (Math|Vector|Normalize _v))
  (bind _returnvalue_3 (Class|KismetMathLibrary|MakeRotfromYZ _returnvalue_2 _returnvalue))
  (bind _returnvalue_4 (* _returnvalue_2 _l))
  (Rendering|Debug|FlushPersistentDebugLines)
  (Rendering|Debug|DrawDebugLine (* _returnvalue_2 (Variables|Default|GetS)) _returnvalue_4 "(R=0.188703,G=0.788491,B=1.000000,A=1.000000)" 9999.0 5.0)
  (AddComponent|AddStaticMeshComponent false (Math|Transform|MakeTransform (+ (* _returnvalue_4 1.05) (* (.Z (Math|Rotator|GetAxes _returnvalue_3)) -15.0)) _returnvalue_3))
  (Rendering|Material|SetScalarParameterValue "/ImpostorBaker/ImpostorBaker/MPC/MPC_ImposterCapture.MPC_ImposterCapture" "EnableCapture" 1.0 :!class /Script/Engine.KismetMaterialLibrary)
  (Rendering|Material|SetScalarParameterValue "/ImpostorBaker/ImpostorBaker/MPC/MPC_ImposterCapture.MPC_ImposterCapture" "Depth" 1.0 :!class /Script/Engine.KismetMaterialLibrary)
  (Rendering|Material|SetScalarParameterValue "/ImpostorBaker/ImpostorBaker/MPC/MPC_ImposterCapture.MPC_ImposterCapture" "R" 1e+03 :!class /Script/Engine.KismetMaterialLibrary)
  (Rendering|Material|SetVectorParameterValue "/ImpostorBaker/ImpostorBaker/MPC/MPC_ImposterCapture.MPC_ImposterCapture" "X" (Math|Color|MakeColor 1.0 0.0 0.0) :!class /Script/Engine.KismetMaterialLibrary)
  (Rendering|Material|SetVectorParameterValue "/ImpostorBaker/ImpostorBaker/MPC/MPC_ImposterCapture.MPC_ImposterCapture" "Y" (Math|Color|MakeColor 0.0 1.0 0.0) :!class /Script/Engine.KismetMaterialLibrary)
  (Rendering|Material|SetVectorParameterValue "/ImpostorBaker/ImpostorBaker/MPC/MPC_ImposterCapture.MPC_ImposterCapture" "Z" (Math|Color|MakeColor 0.0 0.0 1.0) :!class /Script/Engine.KismetMaterialLibrary))