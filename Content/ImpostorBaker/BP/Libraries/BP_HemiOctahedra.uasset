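; Blueprint function library for the Impostor Baker that converts between unit vectors and 2D hemi-octahedral coordinates.
; Encoding takes absolute components, divides by their sum and outputs X+Y and X−Y, so the input's signs are discarded.
; Decoding rotates and halves the 2D coordinates, rebuilds Z as one minus the absolute X and Y, then normalizes.
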(fn UnitVectortoHemiOctahedron
  (params (Unit%20Vector :type Vector))
  (bind (_x _y _z) (Math|Vector|BreakVector Unit%20Vector))
  (bind _returnvalue (Math|Float|Absolute(Float) _x))
  (bind _returnvalue_2 (Math|Float|Absolute(Float) _y))
  (bind _returnvalue_3 (Math|Float|Absolute(Float) _z))
  (bind _returnvalue_4 (Math|Vector|MakeVector _returnvalue _returnvalue_2 _returnvalue_3))
  (bind _returnvalue_5 (Math|Vector|DotProduct _returnvalue_4 "1.000000,1.000000,1.000000"))
  (bind _returnvalue_6 (/ _returnvalue_4 _returnvalue_5))
  (bind (_x_2 _y_2) (Math|Vector|BreakVector _returnvalue_6))
  (return (Math|Vector2D|MakeVector2D (+ _x_2 _y_2) (- _x_2 _y_2))))

(fn HemiOctahedrontoUnitVector
  (params (Hemi%20Octahedron :type Vector%202D%20Structure))
  (bind (_x _y) (Math|Vector2D|BreakVector2D Hemi%20Octahedron))
  (bind _returnvalue (- _x _y))
  (bind _returnvalue_2 (+ _x _y))
  (bind _returnvalue_3 (Math|Vector2D|MakeVector2D _returnvalue_2 _returnvalue))
  (bind _returnvalue_4 (* _returnvalue_3 0.5))
  (bind (_x_2 _y_2) (Math|Vector2D|BreakVector2D _returnvalue_4))
  (return (Math|Vector|Normalize (Math|Vector|MakeVector _x_2 _y_2 (- 1.0 (Math|Vector2D|DotProduct(2D) (Math|Vector2D|MakeVector2D (Math|Float|Absolute(Float) _x_2) (Math|Float|Absolute(Float) _y_2)) "(X=1.000000,Y=1.000000)"))))))