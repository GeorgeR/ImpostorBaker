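; Blueprint vector math library in the Impostor Baker, converting between 3D directions and 2D octahedral coordinates.
; VectorToOctahedron projects by L1 norm, folds the lower hemisphere outward, and also outputs a scalar combining both axes quantized to 16 steps.
; OctahedronToVector reverses the fold and normalizes the result.
; Small Vector2D helpers provide saturate and bias-then-scale, while ClampVector2D is an empty stub.
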(fn VectortoOctahedron
  (params (Vector :type Vector))
  (bind (_x _y _z) (Math|Vector|BreakVector Vector))
  (bind (_x_2 _y_2 _z_2) (Math|Vector|BreakVector Vector))
  (bind _returnvalue (Math|Float|Absolute(Float) _z))
  (bind _returnvalue_2 (Math|Float|Absolute(Float) _x))
  (bind _returnvalue_3 (Math|Float|Absolute(Float) _y))
  (bind _returnvalue_4 (Math|Vector2D|MakeVector2D _x_2 _y_2))
  (bind _returnvalue_5 (Math|Vector|MakeVector _returnvalue_2 _returnvalue_3 _returnvalue))
  (bind _returnvalue_6 (Math|Vector|DotProduct _returnvalue_5 "1.000000,1.000000,1.000000"))
  (bind _returnvalue_7 (/ _returnvalue_4 _returnvalue_6))
  (bind (_x_3 _y_3) (Math|Vector2D|BreakVector2D _returnvalue_7))
  (LocalVariables|Setxy _returnvalue_7)
  (return (select (<= _z_2 0.0) (Math|Vector2D|MakeVector2D (* (Math|Float|SelectFloat 1.0 -1.0 (>= (.X (Math|Vector2D|BreakVector2D (LocalVariables|Getxy))) 0.0)) (- 1.0 (Math|Float|Absolute(Float) _y_3))) (* (Math|Float|SelectFloat 1.0 -1.0 (>= (.Y (Math|Vector2D|BreakVector2D (LocalVariables|Getxy))) 0.0)) (- 1.0 (Math|Float|Absolute(Float) _x_3)))) _returnvalue_7) (+ (/ (Math|Conversions|ToFloat(Integer) (Math|Float|Truncate (* (.X (Math|Vector2D|BreakVector2D (* (+ (select (<= _z_2 0.0) (Math|Vector2D|MakeVector2D (* (Math|Float|SelectFloat 1.0 -1.0 (>= (.X (Math|Vector2D|BreakVector2D (LocalVariables|Getxy))) 0.0)) (- 1.0 (Math|Float|Absolute(Float) _y_3))) (* (Math|Float|SelectFloat 1.0 -1.0 (>= (.Y (Math|Vector2D|BreakVector2D (LocalVariables|Getxy))) 0.0)) (- 1.0 (Math|Float|Absolute(Float) _x_3)))) _returnvalue_7) 1.0) 0.5))) 16.0))) 255.0) (/ (Math|Conversions|ToFloat(Integer) (Math|Float|Truncate (* (.Y (Math|Vector2D|BreakVector2D (* (+ (select (<= _z_2 0.0) (Math|Vector2D|MakeVector2D (* (Math|Float|SelectFloat 1.0 -1.0 (>= (.X (Math|Vector2D|BreakVector2D (LocalVariables|Getxy))) 0.0)) (- 1.0 (Math|Float|Absolute(Float) _y_3))) (* (Math|Float|SelectFloat 1.0 -1.0 (>= (.Y (Math|Vector2D|BreakVector2D (LocalVariables|Getxy))) 0.0)) (- 1.0 (Math|Float|Absolute(Float) _x_3)))) _returnvalue_7) 1.0) 0.5))) 16.0))) 16.0))))

(fn OctahedrontoVector
  (params (Octahedron :type Vector%202D%20Structure))
  (bind (_x _y) (Math|Vector2D|BreakVector2D Octahedron))
  (bind (_x_2 _y_2) (Math|Vector2D|BreakVector2D Octahedron))
  (bind (_x_3 _y_3) (Math|Vector2D|BreakVector2D Octahedron))
  (bind _returnvalue (Math|Float|Absolute(Float) _x_2))
  (bind _returnvalue_2 (Math|Float|Absolute(Float) _y_2))
  (bind _returnvalue_3 (Math|Vector2D|MakeVector2D _returnvalue _returnvalue_2))
  (bind _returnvalue_4 (Math|Vector2D|DotProduct(2D) _returnvalue_3 "(X=1.000000,Y=1.000000)"))
  (bind _returnvalue_5 (- 1.0 _returnvalue_4))
  (return (select (< _returnvalue_5 0.0) (Math|Vector|Normalize (Math|Vector|MakeVector (* (Math|Float|SelectFloat 1.0 -1.0 (>= _x_3 0.0)) (- 1.0 (Math|Float|Absolute(Float) _y_3))) (* (Math|Float|SelectFloat 1.0 -1.0 (>= _y_3 0.0)) (- 1.0 (Math|Float|Absolute(Float) _x_3))) _returnvalue_5)) (Math|Vector|Normalize (Math|Vector|MakeVector _x _y _returnvalue_5)))))

(fn SaturateVector2D
  (params (InVec2D :type Vector%202D%20Structure))
  (bind (_x _y) (Math|Vector2D|BreakVector2D InVec2D))
  (return (Math|Vector2D|MakeVector2D (Math|Float|Clamp(Float) _x) (Math|Float|Clamp(Float) _y))))

(fn BiasScaleVector2D
  (params (InVec2D :type Vector%202D%20Structure) (Bias :type Float%20%28single-precision%29) (Scale :type Float%20%28single-precision%29))
  (return (* (+ InVec2D Bias) Scale)))

(fn ClampVector2D)