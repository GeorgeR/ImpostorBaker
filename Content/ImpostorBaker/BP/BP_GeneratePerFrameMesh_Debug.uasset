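; Impostor baker debug Blueprint that builds a procedural mesh with one quad per frame of a FramesXY grid.
; BuildStaticMesh loops the grid, calling Quad to fill the buffers, then creates the section with M_VSShrink.
; Each origin-centered quad faces its hemi-octahedron direction and maps to its atlas cell in UVs.
; Vertex colors encode grid position and frame index, likely for the material.
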(event Custom|Build%20Static%20Mesh
  (bind _frames_xy (Variables|Default|GetFrames%20XY))
  (bind _frames_xy_2 (Variables|Default|GetFrames%20XY))
  (bind _returnvalue (Math|Conversions|ToFloat(Integer) _frames_xy_2))
  (bind _returnvalue_2 (- _returnvalue 1.0))
  (Utilities|Array|Clear (Variables|Default|GetVerts))
  (Utilities|Array|Clear (Variables|Default|GetTris))
  (Utilities|Array|Clear (Variables|Default|GetUVs))
  (Utilities|Array|Clear (Variables|Default|GetVertColors))
  (Utilities|Array|Clear (Variables|Default|GetNormals))
  (Utilities|Array|Clear (Variables|Default|GetTangents))
  (Utilities|FlowControl|Sequence
    (:then_0
      (bind (_current_point _total_points _0_1_phase _poly_center _x_row _y_row) (Utilities|2DGridExecutionMacro :X _frames_xy :Y _frames_xy)
        (:Per%20Poly%20Execution
          (Variables|Default|SetCurIndex _current_point)
          (Utilities|Quad (- (* (Math|Vector2D|MakeVector2D (/ (Math|Conversions|ToFloat(Integer) _x_row) _returnvalue_2) (/ (Math|Conversions|ToFloat(Integer) _y_row) _returnvalue_2)) 2.0) 1.0) (Math|Conversions|ToFloat(Integer) _x_row) (Math|Conversions|ToFloat(Integer) _y_row)))))
    (:then_1
      (Class|ProceduralMeshComponent|CreateMeshSectionLinearColor (Variables|Default|GetProceduralMesh) 0 (Variables|Default|GetVerts) (Variables|Default|GetTris) (Variables|Default|GetNormals) (Variables|Default|GetUVs) 0 0 0 (Variables|Default|GetVertColors) (Variables|Default|GetTangents) false)
      (Rendering|Material|SetMaterial (Variables|Default|GetProceduralMesh) 0 "/ImpostorBaker/ImpostorBaker/Materials/Debug/M_VSShrink.M_VSShrink"))))

(fn ConstructionScript)